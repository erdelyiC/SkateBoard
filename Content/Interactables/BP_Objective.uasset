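; BP_Objective is an interactable objective with a configurable mesh, a point value and an inspirational phrase.
; Construction applies the chosen static mesh and zeroes the highlight effect's world rotation.
; SetObjectiveActive stores the active state, sizes the highlight's Radius parameter from the mesh's local bounds and toggles the effect.
; Getters expose the active state, phrase and points, with points doubled while the objective is active.
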(fn ConstructionScript
  (Components|StaticMesh|SetStaticMesh (Variables|Default|GetBaseMesh) (Variables|Properties|GetStaticMesh))
  (Transformation|SetWorldRotation (Variables|Default|GetHighlight) "0, 0, 0" false false))

(fn SetObjectiveActive
  (params (IsActive :type Boolean))
  (bind _output_get (Variables|Default|SetIsActiveObjective IsActive))
  (Niagara|SetNiagaraVariable(Float) (Variables|Default|GetHighlight) "Radius" (Math|Vector|VectorLength (.Max (Components|StaticMesh|GetLocalBounds (Variables|Default|GetBaseMesh)))))
  (Components|Activation|SetActive (Variables|Default|GetHighlight) _output_get false)
  (return))

(fn GetIsActive
  (return (Variables|Default|GetIsActiveObjective)))

(fn GetPhrase
  (return (Variables|Properties|GetInspirationalPhrase)))

(fn GetPoints
  (bind _pointvalue (Variables|Properties|GetPointValue))
  (return (select (Variables|Default|GetIsActiveObjective) (* _pointvalue 2) _pointvalue)))