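; Player controller that forwards Enhanced Input actions to the possessed BP_Player pawn.
; Acceleration and steering pass their action values straight through, and releasing steer triggers the pawn's self-righting.
; Jump is two-stage: pressing prepares it and releasing starts it, each only while the pawn is not falling.
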(event Input|EnhancedActionEvents|EnhancedInputActionIA_Accelerate
  (params (ActionValue :type Float%20%28double-precision%29) (ElapsedSeconds :type Float%20%28double-precision%29) (TriggeredSeconds :type Float%20%28double-precision%29) (InputAction :type Input%20Action%20Object%20Reference :default "/Game/Core/IA_Accelerate.IA_Accelerate"))
  (:Triggered
    (Default|Accelerate (.AsBP%20Player (Utilities|Casting|CastToBP_Player (Pawn|GetControlledPawn))) ActionValue)))

(event Input|EnhancedActionEvents|EnhancedInputActionIA_Steer
  (params (ActionValue :type Float%20%28double-precision%29) (ElapsedSeconds :type Float%20%28double-precision%29) (TriggeredSeconds :type Float%20%28double-precision%29) (InputAction :type Input%20Action%20Object%20Reference :default "/Game/Core/IA_Steer.IA_Steer"))
  (bind _returnvalue (Pawn|GetControlledPawn))
  (bind _asbp_player (Utilities|Casting|CastToBP_Player _returnvalue))
  (:Triggered
    (Default|Steer _asbp_player ActionValue))
  (:Completed
    (Default|SelfRight _asbp_player)))

(event Input|EnhancedActionEvents|EnhancedInputActionIA_Jump
  (params (ActionValue :type Boolean) (ElapsedSeconds :type Float%20%28double-precision%29) (TriggeredSeconds :type Float%20%28double-precision%29) (InputAction :type Input%20Action%20Object%20Reference :default "/Game/Core/IA_Jump.IA_Jump"))
  (bind _returnvalue (Pawn|GetControlledPawn))
  (bind _asbp_player (Utilities|Casting|CastToBP_Player _returnvalue))
  (bind _isfalling (Variables|/Game/Character/BP_Player.BP_Player_C|GetIsFalling _asbp_player))
  (:Started
    (if (not _isfalling)
      (Default|PrepareJump _asbp_player)))
  (:Completed
    (if (not _isfalling)
      (Default|StartJump _asbp_player))))

(fn ConstructionScript)